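; BP_Spawn is an Exo VFX Blueprint that rebuilds its spline at BeginPlay, apparently as a test of a procedural helix.
; It removes points by index with debug prints, clears the spline, then adds points in a loop with cosine/sine XY and rising Z.
; The angle factor uses integer division that evaluates to zero, so the points form a straight vertical line.
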(event `self.ReceiveBeginPlay`
  (bind _returnvalue (- (`SplineComponent.GetNumberOfSplinePoints` (`self.Spline`)) 1))
  (`KismetSystemLibrary.PrintString` (`KismetStringLibrary.Conv_IntToString` _returnvalue))
  (for _index (range (+ _returnvalue 1))
    (`SplineComponent.RemoveSplinePoint` (`self.Spline`) _index true)
    (`KismetSystemLibrary.PrintString` (`KismetStringLibrary.Conv_IntToString` _index)))
  (`KismetSystemLibrary.PrintString` "Hello")
  (`SplineComponent.ClearSplinePoints` (`self.Spline`) true)
  (for _index_2 (range 11)
    (bind _returnvalue_2 (`KismetMathLibrary.Conv_IntToDouble` (* _index_2 (/ 3 360))))
    (`SplineComponent.AddPoint` (`self.Spline`) (make `SplinePoint` (`KismetMathLibrary.Conv_IntToDouble` _index_2) (`KismetMathLibrary.MakeVector` (`KismetMathLibrary.DegCos` _returnvalue_2) (`KismetMathLibrary.DegSin` _returnvalue_2) (`KismetMathLibrary.Conv_IntToDouble` (* _index_2 10)))) true)))

(fn `UserConstructionScript`)